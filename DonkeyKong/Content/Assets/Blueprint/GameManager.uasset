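; GameManager blueprint that handles best-score persistence, the game-over transition and barrel cleanup.
; On BeginPlay it loads the BP_SaveData slot or creates a new save object if none exists.
; GoingToGameOver acts at zero lives, saving the score if it matches or beats the best, then opening MAP_GameOver after a short delay.
; CleanMap destroys every BP_Barrel and BP_BarrelBlue actor.
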(event `self.ReceiveBeginPlay`
  (bind _returnvalue (`GameplayStatics.DoesSaveGameExist` (`self.SaveName`)))
  (if _returnvalue
    (`self.LoadData`)
    (else
      (bind _returnvalue_2 (`GameplayStatics.CreateSaveGameObject` "/Game/Assets/Blueprint/BP_SaveData.BP_SaveData_C"))
      (bind _asbp_save_data (cast `/Game/Assets/Blueprint/BP_SaveData` _returnvalue_2))
      (set `self.SaveData` _asbp_save_data))))

(event `GoingToGameOver`
  (if (== (`self.Live`) 0)
    (if (>= (`self.SCORE`) (`/Game/Assets/Blueprint/BP_SaveData.BestScore` (`self.SaveData`)))
      (`self.SaveCurrentData`))
    (`KismetSystemLibrary.Delay` 1.0)
    (`GameplayStatics.OpenLevel` "MAP_GameOver")))

(event `CleanMap`
  (bind _outactors (`GameplayStatics.GetAllActorsOfClass` "/Game/Assets/Blueprint/Obstacle/BP_Barrel.BP_Barrel_C"))
  (for _array_element _outactors
    (`self.K2_DestroyActor` _array_element))
  (bind _outactors_2 (`GameplayStatics.GetAllActorsOfClass` "/Game/Assets/Blueprint/Obstacle/BP_BarrelBlue.BP_BarrelBlue_C"))
  (for _array_element_2 _outactors_2
    (`self.K2_DestroyActor` _array_element_2)))

(fn `LoadData`
  (bind _returnvalue (`GameplayStatics.LoadGameFromSlot` (`self.SaveName`)))
  (bind _asbp_save_data (cast `/Game/Assets/Blueprint/BP_SaveData` _returnvalue))
  (set `self.SaveData` _asbp_save_data)
  (set `self.BESTSCORE` (`/Game/Assets/Blueprint/BP_SaveData.BestScore` (`self.SaveData`)))
  (`KismetSystemLibrary.PrintString` "Data Loaded"))

(fn `SaveCurrentData`
  (set `self.BESTSCORE` (`self.SCORE`))
  (set `/Game/Assets/Blueprint/BP_SaveData.BestScore` (`self.BESTSCORE`) (`self.SaveData`))
  (bind _returnvalue (`GameplayStatics.SaveGameToSlot` (`self.SaveData`) (`self.SaveName`)))
  (`KismetSystemLibrary.PrintString` (`KismetMathLibrary.SelectString` "Save Success" "Save Failed" _returnvalue)))

(fn `UserConstructionScript`)