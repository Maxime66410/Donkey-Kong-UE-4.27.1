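; Barrel generator actor that repeatedly spawns obstacle barrels at its Arrow component's location and launches them.
; After a short delay on BeginPlay, it picks one of the first two ObstacleType classes at random.
; BP_Barrel gets a fixed world +Y and upward impulse, while BP_BarrelBlue gets a random sideways Y with the same lift.
; Each successful launch resets the spawn timer to a new random interval.
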(event `self.ReceiveBeginPlay`
  (`KismetSystemLibrary.K2_SetTimerDelegate` (delegate `SpawnBarrel`) 2.0))

(event `SpawnBarrel`
  (bind _returnvalue (`|SpawnActorFromClass` (`|GetArrayItem` (`self.ObstacleType`) (`KismetMathLibrary.RandomIntegerInRange` 0 1)) (`KismetMathLibrary.Conv_VectorToTransform` (`SceneComponent.K2_GetComponentLocation` (`self.Arrow`))) "AdjustIfPossibleButAlwaysSpawn" "OverrideRootScale" null null))
  (bind _asbp_barrel (cast `/Game/Assets/Blueprint/Obstacle/BP_Barrel` _returnvalue)
    (:`then`
      (`PrimitiveComponent.AddImpulse` (`/Game/Assets/Blueprint/Obstacle/BP_Barrel.Capsule` _asbp_barrel) (0.0 500.0 500.0) "None" true))
    (:`CastFailed`
      (bind _asbp_barrel_blue (cast `/Game/Assets/Blueprint/Obstacle/BP_BarrelBlue` _returnvalue))
      (`PrimitiveComponent.AddImpulse` (`/Game/Assets/Blueprint/Obstacle/BP_BarrelBlue.Capsule` _asbp_barrel_blue) (`KismetMathLibrary.MakeVector` 0.0 (`KismetMathLibrary.RandomFloatInRange` -500.0 500.0) 500.0) "None" true)))
  (set `self.RandomRestart` (`KismetMathLibrary.RandomFloatInRange` 0.5 3.0))
  (`KismetSystemLibrary.K2_SetTimerDelegate` (delegate `SpawnBarrel`) (`self.RandomRestart`) true))

(fn `UserConstructionScript`)